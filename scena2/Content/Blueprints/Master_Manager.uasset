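; Master_Manager switches between a Blueprint and a C++ controller actor, or turns both off.
; B flips the active implementation and N toggles both on or off, each printing the new state in Polish.
; SetActiveManager applies the state through actor tick, also toggling component ticks on the C++ controller only.
; BeginPlay applies the initial state and copies its RenderDistance to both controllers.
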(event EventBeginPlay
  (bind _render_distance (Variables|Default|GetRender%20Distance))
  (CallFunction|SetActiveManager)
  (bind _ascontroller_bp (Utilities|Casting|CastToController_BP (Variables|Default|Getcontroller_bp)))
  (Variables|/Game/Blueprints/Controller_BP.Controller_BP_C|SetrenderDistance _ascontroller_bp _render_distance)
  (bind _ascontroller_cpp (Utilities|Casting|CastToController_CPP (Variables|Default|Getcontroller_cpp)))
  (Variables|/Script/scena2_blueprint.Controller_CPP|SetRenderDistance _ascontroller_cpp _render_distance))

(event Collision|EventActorBeginOverlap
  (params (OtherActor :type Actor%20Object%20Reference)))

(event EventTick
  (params (DeltaSeconds :type Float%20%28single-precision%29)))

(event Input|KeyboardEvents|B
  (params (Key :type Key%20Structure :default "None"))
  (:Pressed
    (Variables|Default|Setblueprint_active (not (Variables|Default|Getblueprint_active)))
    (CallFunction|SetActiveManager)
    (Development|PrintString (Utilities|String|Append (Utilities|String|SelectString "Kontroler: blueprint, " "Kontroler: CPP, " (Variables|Default|Getblueprint_active)) (Utilities|String|SelectString "Kontrolery: ON" "Kontrolery: OFF" (Variables|Default|Getcontrollers_on))))))

(event Input|KeyboardEvents|N
  (params (Key :type Key%20Structure :default "None"))
  (:Pressed
    (Variables|Default|Setcontrollers_on (not (Variables|Default|Getcontrollers_on)))
    (CallFunction|SetActiveManager)
    (Development|PrintString (Utilities|String|Append (Utilities|String|SelectString "Kontroler: blueprint, " "Kontroler: CPP, " (Variables|Default|Getblueprint_active)) (Utilities|String|SelectString "Kontrolery: ON" "Kontrolery: OFF" (Variables|Default|Getcontrollers_on))))))

(fn ConstructionScript)

(fn SetActiveManager
  (bind _controller_bp (Variables|Default|Getcontroller_bp))
  (bind _controller_cpp (Variables|Default|Getcontroller_cpp))
  (bind _returnvalue (Actor|GetComponentsByClass _controller_cpp "/Script/Engine.ActorComponent"))
  (if (Variables|Default|Getcontrollers_on)
    (if (Variables|Default|Getblueprint_active)
      (Actor|Tick|SetActorTickEnabled _controller_bp true)
      (Actor|Tick|SetActorTickEnabled _controller_cpp)
      (for _array_element _returnvalue :!label _label
        (Components|Tick|SetComponentTickEnabled _array_element false))
      (else
        (Actor|Tick|SetActorTickEnabled _controller_bp)
        (Actor|Tick|SetActorTickEnabled _controller_cpp true)
        (for _array_element_2 _returnvalue
          (Components|Tick|SetComponentTickEnabled _array_element_2 true))))
    (else
      (Actor|Tick|SetActorTickEnabled _controller_bp)
      (Actor|Tick|SetActorTickEnabled _controller_cpp)
      (goto _label))))