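; Benchmark actor that measures how long Blueprint takes to repeatedly average an array of random floats.
; Each Tick runs one summing pass; when the repeat count runs out, it adds the Timer_BP actor's elapsed time to a total and re-randomizes the array.
; After all test iterations, it broadcasts the mean iteration time through OnBenchmarkCompleteBp2, with trace bookmarks marking start and end.
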(event EventBeginPlay
  ;[0.15 0.15 0.15 0.5] Zdarzenie BeginPlay
  (bind _outactors (Actor|GetAllActorsOfClass "/Game/Blueprints/Timer_BP.Timer_BP_C"))
  (Variables|Default|SettimerActor (Utilities|Array|Get(acopy) _outactors))
  (Class|TraceUtilLibrary|TraceBookmark "Benchmark BP2 start")
  (Variables|Default|Settotaliterations (Variables|Default|GetTestIterations))
  ;;[0.15 0.15 0.15 0.5] Inicjalizacja tablicy
  (Variables|Default|SettotalRepeats (Variables|Default|GetRepeat))
  (Utilities|Array|Clear (Variables|Default|GetArray))
  (for _index (range 0 (Variables|Default|GetArraySize))
    (Utilities|Array|Add (Variables|Default|GetArray) (Math|Random|RandomFloatinRange 0.0 1.0))))

(event Collision|EventActorBeginOverlap
  (params (OtherActor :type Actor%20Object%20Reference)))

(event EventTick
  (params (DeltaSeconds :type Float%20%28single-precision%29))
  (bind _testiterations (Variables|Default|GetTestIterations))
  ;[0.15 0.15 0.15 0.5] Sprawdzenie nowej iteracji
  (if (Variables|Default|GetnewIteration)
    (Variables|Default|SetnewIteration false)
    (Class|Timer|StartTimer (Variables|Default|GettimerActor)))
  ;[0.15 0.15 0.15 0.5] Pojedyncza iteracja obliczenia średniej
  (if (> (Variables|Default|GetRepeat) 0)
    (Math|Integer|DecrementInt (Variables|Default|GetRepeat)
      (:%20%20
        (Variables|Default|Setsum 0.0)
        (for _index (range 0 (Variables|Default|GetArraySize))
          (Variables|Default|Setsum (+ (Variables|Default|Getsum) (Utilities|Array|Get(acopy) (Variables|Default|GetArray) _index))))
        (Variables|Default|Setavg (/ (Variables|Default|Getsum) (Variables|Default|GetArraySize)))))
    (else
      ;[0.15 0.15 0.15 0.5] Sprawdzenie liczby iteracji
      (if (> _testiterations 0)
        (Math|Integer|DecrementInt _testiterations
          (:%20%20
            ;[0.15 0.15 0.15 0.5] zapis czasu trwania iteracji
            (bind _returnvalue (Class|Timer|StopTimer (Variables|Default|GettimerActor)))
            (Variables|Default|Settotaltime (+ _returnvalue (Variables|Default|Gettotaltime)))
            ;[0.15 0.15 0.15 0.5] losowanie tablicy
            (Variables|Default|SetRepeat (Variables|Default|GettotalRepeats))
            (Utilities|Array|Clear (Variables|Default|GetArray))
            (for _index_2 (range 0 (Variables|Default|GetArraySize))
              (Utilities|Array|Add (Variables|Default|GetArray) (Math|Random|RandomFloatinRange 0.0 1.0)))
            (Variables|Default|SetnewIteration true)))
        (else
          ;[0.15 0.15 0.15 0.5] warunek końca testu
          (if (and (not (Variables|Default|Getfinished)) (<= (Variables|Default|GetTestIterations) 0))
            ;[0.15 0.15 0.15 0.5] koniec testu
            (Variables|Default|Setfinished true)
            (Class|TraceUtilLibrary|TraceBookmark "Benchmark BP2 end")
            (Variables|Default|SetnewIteration false)
            (bind _output_get (Variables|Default|Setavgtime (/ (Variables|Default|Gettotaltime) (Variables|Default|Gettotaliterations))))
            (Default|CallOnBenchmarkCompleteBp2 _output_get)))))))

(fn ConstructionScript)