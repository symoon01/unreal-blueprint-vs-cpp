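; Blueprint benchmark actor that times averaging a random float array over a number of test iterations.
; Each Tick runs one iteration: it refills the array, then times repeated sum-and-divide loops through a Timer_BP actor found at BeginPlay.
; When iterations run out, it divides total time by the initial count plus one and fires OnBenchmarkCompleteBp.
; Trace bookmarks mark the benchmark's start and end.
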(event EventBeginPlay
  ;[0.15 0.15 0.15 0.5] zdarzenie BeginPlay
  (bind _outactors (Actor|GetAllActorsOfClass "/Game/Blueprints/Timer_BP.Timer_BP_C"))
  (Variables|Default|SettimerActor (Utilities|Array|Get(acopy) _outactors))
  (Class|TraceUtilLibrary|TraceBookmark "Benchmark BP start")
  (Variables|Default|Settotaliterations (+ (Variables|Default|GetTestIterations) 1)))

(event Collision|EventActorBeginOverlap
  (params (OtherActor :type Actor%20Object%20Reference)))

(event EventTick
  (params (DeltaSeconds :type Float%20%28single-precision%29))
  ;[0.15 0.15 0.15 0.5] początek iteracji
  (if (> (Variables|Default|GetTestIterations) 0)
    (bind _result (Math|Integer|DecrementInt (Variables|Default|GetTestIterations))
      (:%20%20
        ;[0.15 0.15 0.15 0.5] Losowanie tablicy i ustawienie Timera
        (Variables|Default|SetTestIterations _result)
        (Utilities|Array|Clear (Variables|Default|GetArray))
        (for _index (range 0 (Variables|Default|GetArraySize))
          (Utilities|Array|Add (Variables|Default|GetArray) (Math|Random|RandomFloatinRange 0.0 1.0)))
        (Class|Timer|StartTimer (Variables|Default|GettimerActor))
        ;[0.15 0.15 0.15 0.5] Pętle liczenia sredniej
        (for _index_2 (range 0 (Variables|Default|GetRepeat))
          (Variables|Default|Setsum 0.0)
          (for _index_3 (range 0 (Variables|Default|GetArraySize))
            (Variables|Default|Setsum (+ (Variables|Default|Getsum) (Utilities|Array|Get(acopy) (Variables|Default|GetArray) _index_3))))
          (Variables|Default|Setavg (/ (Variables|Default|Getsum) (Variables|Default|GetArraySize))))
        ;[0.15 0.15 0.15 0.5] Zakończenie iteracji
        (bind _returnvalue (Class|Timer|StopTimer (Variables|Default|GettimerActor)))
        (Variables|Default|Settotaltime (+ _returnvalue (Variables|Default|Gettotaltime)))))
    (elif (not (Variables|Default|Getfinished))
      ;[0.15 0.15 0.15 0.5] Zakończenie testu
      (bind _output_get (Variables|Default|Setavgtime (/ (Variables|Default|Gettotaltime) (Variables|Default|Gettotaliterations))))
      (Default|CallOnBenchmarkCompleteBp _output_get)
      (Variables|Default|Setfinished true)
      (Class|TraceUtilLibrary|TraceBookmark "Benchmark BP end"))))

(fn ConstructionScript)