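; Robot pawn that wanders by itself in random horizontal directions and picks random arm poses.
; BeginPlay runs both randomizers once, then starts looping timers by function name, with the movement direction changing less often than the arm rotation.
; Tick feeds the stored Direction into AddMovementInput every frame.
; NewArmRotation receives a random pitch and yaw with zero roll, but nothing in this graph applies it.
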(event EventBeginPlay
  (CallFunction|ChangeDirection)
  (Utilities|Time|SetTimerbyFunctionName 0 "ChangeDirection" 5.0 true)
  (CallFunction|ChangeHandRotation)
  (Utilities|Time|SetTimerbyFunctionName 0 "ChangeHandRotation" 1.0 true))

(event Collision|EventActorBeginOverlap
  (params (OtherActor :type Actor%20Object%20Reference)))

(event EventTick
  (params (DeltaSeconds :type Float%20%28single-precision%29))
  (Pawn|Input|AddMovementInput (Variables|Default|Getdirection) 1.0 false))

(fn ConstructionScript)

(fn ChangeDirection
  (Variables|Default|Setdirection (Math|Vector|MakeVector (Math|Random|RandomFloatinRange -1.0 1.0) (Math|Random|RandomFloatinRange -1.0 1.0) 0.0)))

(fn ChangeHandRotation
  (Variables|Default|SetnewArmRotation (Math|Rotator|MakeRotator 0.0 (Math|Random|RandomFloatinRange 0.0 9e+01) (Math|Random|RandomFloatinRange -9e+01 9e+01))))