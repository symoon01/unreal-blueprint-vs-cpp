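; Robot spawner actor that populates the level with a configurable number of Robot instances when play begins.
; A BeginPlay loop spawns each one at a random X/Y within the spawn area range around the world origin, at a fixed height and independent of the spawner's location.
; Each valid robot then gets its default controller through SpawnDefaultController.
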(event EventBeginPlay
  (bind _spawnarearange (Variables|Default|GetspawnAreaRange))
  (bind _returnvalue (* _spawnarearange -1.0))
  (for _index (range 1 (Variables|Default|GetnumRobots))
    (bind _returnvalue_2 (Game|SpawnActorfromClass "/Game/Blueprints/Robot.Robot_C" (Math|Transform|MakeTransform (Math|Vector|MakeVector (Math|Random|RandomFloatinRange _spawnarearange _returnvalue) (Math|Random|RandomFloatinRange _spawnarearange _returnvalue) 2e+02)) "Undefined" "MultiplyWithRoot" 0 0))
    (Utilities|IsValid _returnvalue_2
      (:Is%20Valid
        (Pawn|SpawnDefaultController _returnvalue_2)))))

(event Collision|EventActorBeginOverlap
  (params (OtherActor :type Actor%20Object%20Reference)))

(event EventTick
  (params (DeltaSeconds :type Float%20%28single-precision%29)))

(fn ConstructionScript)